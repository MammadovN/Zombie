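; PlayerDeathActor is a physics-driven actor that, judging by its name, stands in for the player on death.
; On BeginPlay it copies stored settings into its post-process component and gives its Cube a randomized horizontal impulse.
; The impulse point is also random and absolute, not offset from the actor's position.
; A coin flip then fires either the left or right force component for an extra kick.
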(event `self.ReceiveBeginPlay`
  (bind _returnvalue (`KismetMathLibrary.RandomFloatInRange` -10.0 10.0))
  (bind _returnvalue_2 (* (`KismetMathLibrary.MakeVector` _returnvalue _returnvalue) 650.0))
  (set `PostProcessComponent.Settings` (`self.PPSetings`) (`self.PostProcess`))
  (`PrimitiveComponent.AddImpulseAtLocation` (`self.Cube`) _returnvalue_2 _returnvalue_2 "None")
  (if (`KismetMathLibrary.RandomBool`)
    (`RadialForceComponent.FireImpulse` (`self.LeftForce`))
    (else
      (`RadialForceComponent.FireImpulse` (`self.RightForce`)))))

(fn `UserConstructionScript`)