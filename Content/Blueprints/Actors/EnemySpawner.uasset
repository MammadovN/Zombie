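; Enemy spawner actor that creates a zombie AI character at its own location whenever its SpawnZombie event is called.
; Each spawn runs AI_BehaviourTree, ignores collision failure and increments the zombie count on the cached FPS_GameState.
; The new zombie receives the world position of the StartGoalLocation component as its initial goal.
; The construction script places that component from the GoalVector and GoalRotation variables, relative to its parent.
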(event `self.ReceiveBeginPlay`
  (bind _asfps_game_state (cast `/Game/Blueprints/FPS_GameState` (`GameplayStatics.GetGameState`)))
  (set `self.GameStateRef` _asfps_game_state))

(event `SpawnZombie`
  (bind _returnvalue (`AIBlueprintHelperLibrary.SpawnAIFromClass` "/Game/AI/AI_Character_Child.AI_Character_Child_C" "/Game/AI/AI_BehaviourTree.AI_BehaviourTree" (`self.K2_GetActorLocation`) (`self.K2_GetActorRotation`) true null))
  (`/Engine/EditorBlueprintResources/StandardMacros.IncrementInt` (`/Game/Blueprints/FPS_GameState.NumberOfZombies` (`self.GameStateRef`))
    (:`  `
      (bind _asai_character_child (cast `/Game/AI/AI_Character_Child` _returnvalue))
      (set `/Game/AI/AI_Character.StartGoalLocation` (`SceneComponent.K2_GetComponentLocation` (`self.StartGoalLocation`)) _asai_character_child))))

(fn `UserConstructionScript`
  (`SceneComponent.K2_SetRelativeLocationAndRotation` (`self.StartGoalLocation`) (`self.GoalVector`) (`self.GoalRotation`) false false))