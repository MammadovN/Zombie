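; Grenade launcher weapon Blueprint built on a parent weapon class.
; On BeginPlay it runs the parent setup, then pulls its grenade launcher ammo data from the FPS game instance.
; On fire it runs the parent firing logic and plays the launcher's fire animation once on the gun mesh.
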(event `self.ReceiveBeginPlay`
  (`parent.ReceiveBeginPlay`)
  (bind _asfps_game_instance (cast `/Game/Blueprints/FPS_GameInstance` (`GameplayStatics.GetGameInstance`)))
  (set `self.AmmoData` (`/Game/Blueprints/FPS_GameInstance.GrenadeLauncherAmmoData` _asfps_game_instance)))

(event `self.WeaponFire`
  (params (FireType :type "/Game/Blueprints/Enums/FireType Enum" :default "NewEnumerator0"))
  (`parent.WeaponFire` FireType)
  (`SkeletalMeshComponent.PlayAnimation` (`self.GunMesh`) "/Game/MilitaryWeapSilver/Weapons/Animations/Fire_GrenadeLauncher_W.Fire_GrenadeLauncher_W" false))

(fn `UserConstructionScript`
  (`parent.UserConstructionScript`))