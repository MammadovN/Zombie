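; Assault rifle weapon Blueprint that adds automatic fire to its parent weapon class and loads its ammo data from the FPS game instance.
; WeaponFire shoots immediately, then starts a looping timer at the automatic fire rate.
; Each shot runs the parent fire logic, plays the gun animation and notifies the player character.
; StopFire clears the timer, and an empty magazine stops firing and triggers the player's reload.
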(event `self.ReceiveBeginPlay`
  (`parent.ReceiveBeginPlay`)
  (bind _asfps_game_instance (cast `/Game/Blueprints/FPS_GameInstance` (`GameplayStatics.GetGameInstance`)))
  (set `self.AmmoData` (`/Game/Blueprints/FPS_GameInstance.AssaultRifleAmmoData` _asfps_game_instance)))

(event `self.WeaponFire`
  (params (FireType :type "/Game/Blueprints/Enums/FireType Enum" :default "NewEnumerator0"))
  (set `self.IsRifleFiring?` true)
  (`self.RifleFire`)
  (bind _returnvalue (`KismetSystemLibrary.K2_SetTimerDelegate` (delegate `RifleFire`) (`self.AutomaticFireRate`) true))
  (set `self.RifleFireTimerHandle` _returnvalue))

(event `RifleFire`
  (if (`self.IsRifleFiring?`)
    (`parent.WeaponFire` (stale `self.WeaponFire` FireType))
    (`SkeletalMeshComponent.PlayAnimation` (`self.GunMesh`) "/Game/MilitaryWeapSilver/Weapons/Animations/Fire_Rifle_W.Fire_Rifle_W" false)
    (`/Game/Blueprints/FPS_Character.CharacterFireWeapon` (`self.PlayerRef`) "NewEnumerator1")
    (if (<= (`self.CurrentAmmo`) 0)
      (`self.StopFire`)
      (`/Game/Blueprints/FPS_Character.Reload` (`self.PlayerRef`)))))

(event `self.StopFire`
  (`parent.StopFire`)
  (set `self.IsRifleFiring?` false)
  (`KismetSystemLibrary.K2_ClearAndInvalidateTimerHandle` (`self.RifleFireTimerHandle`)))

(fn `UserConstructionScript`
  (`parent.UserConstructionScript`))